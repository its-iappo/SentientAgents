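; Test character for exercising a HealthComponent through debug input and on-screen output.
; The D key heals shield and the E key heals health by the character's configured amounts, printing each amount.
; Taking any damage briefly prints the component's current health.
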(event EventBeginPlay)

(event Collision|EventActorBeginOverlap
  (params (OtherActor :type Actor%20Object%20Reference)))

(event EventTick
  (params (DeltaSeconds :type Float%20%28single-precision%29)))

(event Game|Damage|EventAnyDamage
  (params (Damage :type Float%20%28single-precision%29) (DamageType :type Damage%20Type%20Object%20Reference) (InstigatedBy :type Controller%20Object%20Reference) (DamageCauser :type Actor%20Object%20Reference))
  (Development|PrintString (Utilities|String|ToString(Float) (Variables|/Script/SentientAgents.HealthComponent|GetCurrentHealth (Variables|Default|GetHealthComponent))) true true "(R=0.000000,G=0.660000,B=1.000000,A=1.000000)" 0.75))

(event Input|KeyboardEvents|E
  (params (Key :type Key%20Structure :default "None"))
  (bind _heal_health (Variables|Default|GetHeal%20Health))
  (:Pressed
    (Class|HealthComponent|HealHealth (Variables|Default|GetHealthComponent) _heal_health)
    (Development|PrintString (Utilities|String|ToString(Float) _heal_health))))

(event Input|KeyboardEvents|D
  (params (Key :type Key%20Structure :default "None"))
  (bind _heal_shield (Variables|Default|GetHeal%20Shield))
  (:Pressed
    (Class|HealthComponent|HealShield (Variables|Default|GetHealthComponent) _heal_shield)
    (Development|PrintString (Utilities|String|ToString(Float) _heal_shield))))

(fn ConstructionScript)